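; Actor Blueprint that melts away by shrinking until it destroys itself, gated by a MeltMe flag.
; BeginPlay clears the flag, and nothing in these graphs sets it to true.
; While it is set, each Tick scales the actor down by a constant factor, independent of delta time, and destroys it once Z scale falls below a small threshold.
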(event `self.ReceiveBeginPlay`
  (set `self.MeltMe` false))

(event `self.ReceiveTick`
  (params (DeltaSeconds :type "Float (single-precision)"))
  (bind _returnvalue (`self.GetActorRelativeScale3D`))
  (if (`self.MeltMe`)
    (`self.SetActorRelativeScale3D` (* _returnvalue 0.95))
    (if (< (.z _returnvalue) 0.1)
      (`self.K2_DestroyActor`))))

(fn `UserConstructionScript`)